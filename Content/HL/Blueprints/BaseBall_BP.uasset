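; BaseBall_BP is a ball actor that reacts the first time the player hits it.
; The Hit event checks that the other component carries the Player tag and that a HitByPlayer flag is still unset.
; HitByPlayer then sets the flag, prints a debug string, enables gravity on the Sphere and calls Effect, which spawns an explosion particle at the actor's transform.
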(event `self.ReceiveActorBeginOverlap`
  (params (OtherActor :type "Actor Object Reference")))

(event `self.ReceiveHit`
  (params (MyComp :type "PrimitiveComponent Object Reference") (Other :type "Actor Object Reference") (OtherComp :type "PrimitiveComponent Object Reference") (bSelfMoved :type Boolean) (HitLocation :type "Vector Structure") (HitNormal :type "Vector Structure") (NormalImpulse :type "Vector Structure") (Hit :type "HitResult Structure (by ref)"))
  (if (`self._HitByPlayer`)
    _
    (elif (`ActorComponent.ComponentHasTag` OtherComp "Player")
      (`self.HitByPlayer`))))

(fn `Effect`
  (bind (_returnvalue_location _returnvalue_rotation _returnvalue_scale) (`KismetMathLibrary.BreakTransform` (`self.GetTransform`)))
  (`GameplayStatics.SpawnEmitterAtLocation` "/Game/StarterContent/Particles/P_Explosion.P_Explosion" _returnvalue_location _returnvalue_rotation _returnvalue_scale))

(fn `HitByPlayer`
  (set `self._HitByPlayer` true)
  (`KismetSystemLibrary.PrintString` "Sphere Hit")
  (`PrimitiveComponent.SetEnableGravity` (`self.Sphere`) true)
  (`self.Effect`))

(fn `UserConstructionScript`)