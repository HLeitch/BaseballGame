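; Player Blueprint that swings a baseball bat, with bat movement by mouse still unfinished.
; Releasing Space plays the BaseballBat component's animation once, without looping.
; Tick calls MoveBat, which currently only prints the mouse's screen position for debugging.
; A camera-forward object trace and a screen-to-world deprojection sit in MoveBat but are not connected.
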(event `self.ReceiveTick`
  (params (DeltaSeconds :type "Float (single-precision)"))
  (`self.Move Bat`))

(event `Key|SpaceBar`
  (params (Key :type "Key Structure"))
  (:`Released`
    (`SkeletalMeshComponent.Play` (`self.BaseballBat`) false)))

(fn `Move Bat`
  (bind (_locationx _locationy) (`PlayerController.GetMousePosition` (`GameplayStatics.GetPlayerController` 0)))
  (`KismetSystemLibrary.PrintString` (`KismetStringLibrary.Concat_StrStr` "Mouse Position: " (`KismetStringLibrary.Conv_Vector2dToString` (`KismetMathLibrary.MakeVector2D` _locationx _locationy))) true true (struct :`G` 0.66 :`B` 1.0 :`A` 1.0) 2.0 "MousePos"))

(fn `UserConstructionScript`)